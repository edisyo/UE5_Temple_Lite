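; BP_EndMountain is the game's ending mountain, which greens its sandstone and leads into the ending sequence when activated.
; A GreenTransition timeline drives the dynamic material blend and lerps the post-process exposure from its saved original toward an end value.
; Timeline events fade out background, ambient and laser audio, then show the ending UI and load the main menu after a delay.
; Deactivate reverses the timeline and fades the aura sound.
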(event `self.ReceiveBeginPlay`
  ;[1 0.5354 0.6876] Initial setup
  (bind _returnvalue (`PrimitiveComponent.CreateDynamicMaterialInstance` (`self.StaticMesh`) 0 "/Game/Materials/MI_Gigantic_Sandstone_Terrain_GREEN.MI_Gigantic_Sandstone_Terrain_GREEN" "None"))
  (set `self.Mat_ref` _returnvalue)
  (bind _outactors (`GameplayStatics.GetAllActorsOfClass` "/Script/Engine.PostProcessVolume"))
  (bind _output_get (set `self.Post_Process_ref` (`|GetArrayItem` _outactors)))
  (set `self.OriginalExposureValue` (`.AutoExposureBias` (break `PostProcessSettings` (`PostProcessVolume.Settings` _output_get)))) ; save original exposure
)

(event `/Game/Blueprints/BPI_Activatable.Activate`
  (`AudioComponent.FadeIn` (`self.aura2`) 2.0 0.5 0.0 "Linear")
  (bind (_direction _material_blend_amount _exposure_lerp_amount) (`Timeline|Green Transition` :!label _label)
    (:`Update`
      ;[1 0.7326 0.3281] Update - Lerping
      (`MaterialInstanceDynamic.SetScalarParameterValue` (`self.Mat_ref`) "Blend_amount" _material_blend_amount)
      (setmembers `PostProcessSettings` :`StructRef` (`PostProcessVolume.Settings` (`self.Post_Process_ref`)) :`AutoExposureBias` (`KismetMathLibrary.Lerp` (`self.OriginalExposureValue`) (`self.EndExposureValue`) _exposure_lerp_amount)))
    (:`SoundFade`
      ;[0.2031 0.3296 1] Fade out audio
      (`AudioComponent.FadeOut` (`self.aura2`) 5.0 0.0 "Linear")
      (`AudioComponent.FadeOut` (`/Game/Blueprints/BP_FirstPersonGameMode.BackgroundAudio` (cast `/Game/Blueprints/BP_FirstPersonGameMode` (`GameplayStatics.GetGameMode`) :!pure true)) 6.0 0.0 "Linear")
      (bind _outactors (`GameplayStatics.GetAllActorsOfClass` "/Script/Engine.AmbientSound"))
      (for _array_element _outactors
        (`AudioComponent.FadeOut` (`AmbientSound.AudioComponent` _array_element) 5.0 0.0 "Linear"))
      (bind _outactors_2 (`GameplayStatics.GetAllActorsOfClass` "/Game/Blueprints/BP_LaserCreator.BP_LaserCreator_C"))
      (for _array_element_2 _outactors_2
        (`AudioComponent.FadeOut` (`/Game/Blueprints/BP_LaserCreator.Audio` _array_element_2) 5.0 0.0 "Linear")))
    (:`Ending`
      (bind _returnvalue (`|CreateWidget` "/Game/CutScenes/WB_EndingUI.WB_EndingUI_C"))
      (`UserWidget.AddToViewport` _returnvalue 0)
      (`KismetSystemLibrary.Delay` 25.0) ; delay for movies length
      (`GameplayStatics.OpenLevelBySoftObjectPtr` "/Game/Maps/MAP_MainMenu.MAP_MainMenu"))))

(event `/Game/Blueprints/BPI_Activatable.Deactivate`
  (`AudioComponent.FadeOut` (`self.aura2`) 2.0 0.0 "Linear") ; Volume level - to what level fade out!!!
  (goto _label :!via `Reverse`))

(fn `UserConstructionScript`)