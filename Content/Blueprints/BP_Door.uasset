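; BP_Door is a sliding door that opens on Activate and, unless ActivateOnce is set, closes on Deactivate.
; Timelines drive the door's relative location from zero to OpeningDistance along the OpenDirection component's local forward vector.
; The reversible DoorOpen timeline uses DoorOpenSpeed as play rate and ends the rock-push loop with a thud.
; The ActivateOnce path uses a separate timeline without that rate or sound ending.
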(event `self.ReceiveBeginPlay`
  ;[1 1 1] Speed up or slow down playrate
  (`TimelineComponent.SetPlayRate` (`self.DoorOpen`) (`self.Door open speed`)))

(event `/Game/Blueprints/BPI_Activatable.Activate`
  ;[1 1 1] Door animation
  (`AudioComponent.FadeIn` (`self.PushRock_loop`) 0.1 1.0 0.0 "Linear")
  (if (`self.ActivateOnce?`)
    (bind (_direction _amount) (`Timeline|Timeline`)
      (:`Update`
        (`SceneComponent.K2_SetRelativeLocation` (`self.Door`) (* (`KismetMathLibrary.Lerp` 0.0 (`self.Opening Distance`) _amount) (`KismetMathLibrary.GetForwardVector` (`SceneComponent.RelativeRotation` (`self.OpenDirection`)))) false false)))
    (else
      (bind (_direction_2 _amount_2) (`Timeline|DoorOpen` :!label _label)
        (:`Update`
          (`SceneComponent.K2_SetRelativeLocation` (`self.Door`) (* (`KismetMathLibrary.Lerp` 0.0 (`self.Opening Distance`) _amount_2) (`KismetMathLibrary.GetForwardVector` (`SceneComponent.RelativeRotation` (`self.OpenDirection`)))) false false))
        (:`Finished`
          (`AudioComponent.FadeOut` (`self.PushRock_loop`) 0.1 0.0 "Linear")
          (`AudioComponent.Play` (`self.RockThud`) 0.1))))))

(event `/Game/Blueprints/BPI_Activatable.Deactivate`
  ;[1 1 1] Door animation
  (`AudioComponent.FadeIn` (`self.PushRock_loop`) 0.1 1.0 0.0 "Linear")
  (if (not (`self.ActivateOnce?`))
    (goto _label :!via `Reverse`)))

(fn `UserConstructionScript`)