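; BP_SpinDoor is a door that rotates open when activated and reverses when deactivated, with a looping gear sound during movement.
; A timeline, paced by DoorOpenSpeed, lerps the Column's yaw from zero to that of an arrow component marking the end rotation.
; On activation, a sphere trace around the door wakes nearby physics-simulating components so they respond to the moving door.
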(event `self.ReceiveBeginPlay`
  (`TimelineComponent.SetPlayRate` (`self.SpinDoor_Animation`) (`self.Door open speed`)))

(event `/Game/Blueprints/BPI_Activatable.Activate`
  (bind (_relativerotation_roll _relativerotation_pitch _relativerotation_yaw) (`KismetMathLibrary.BreakRotator` (`SceneComponent.RelativeRotation` (`self.Arrow_EndRoation`))))
  (`AudioComponent.FadeIn` (`self.GearTurnLoop`) 0.1 1.0 0.0 "Linear")
  (`self.WakeNearByObjects`)
  (bind (_direction _amount) (`Timeline|SpinDoor_Animation` :!label _label)
    (:`Update`
      (`SceneComponent.K2_SetRelativeRotation` (`self.column`) (`KismetMathLibrary.MakeRotator` 0.0 0.0 (`KismetMathLibrary.Lerp` 0.0 _relativerotation_yaw _amount)) false false))
    (:`Finished`
      (`AudioComponent.FadeOut` (`self.GearTurnLoop`) 0.0 0.0 "Linear"))))

(event `/Game/Blueprints/BPI_Activatable.Deactivate`
  (`AudioComponent.FadeIn` (`self.GearTurnLoop`) 0.1 1.0 0.0 "Linear")
  (goto _label :!via `Reverse`))

(fn `UserConstructionScript`)

(fn `WakeNearByObjects`
  (bind _returnvalue (`SceneComponent.K2_GetComponentLocation` (`self.Door`)))
  (bind _outhits (`KismetSystemLibrary.SphereTraceMulti` _returnvalue _returnvalue 350.0 "TraceTypeQuery1"))
  (for _array_element _outhits
    (bind (_bblockinghit _binitialoverlap _time _distance _location _impactpoint _normal _impactnormal _physmat _hitactor _hitcomponent) (`GameplayStatics.BreakHitResult` _array_element))
    (if (`SceneComponent.IsSimulatingPhysics` _hitcomponent "None")
      (`PrimitiveComponent.WakeAllRigidBodies` _hitcomponent))))