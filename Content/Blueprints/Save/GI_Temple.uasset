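; GI_Temple is the game instance that owns the persistent save data for checkpoints and player settings.
; On Init it loads BP_SaveData from the main save slot, or creates a fresh save object if none exists.
; Save events for checkpoint, sensitivity, final gather and scene detail each update their field on that object and immediately write it back to the slot.
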(event `self.ReceiveInit`
  ;[1 1 1] Creating a SAVE GAME DATA on game Startup
  (bind _returnvalue (`GameplayStatics.DoesSaveGameExist` "MainSlot"))
  (if _returnvalue
    (bind _returnvalue_2 (`GameplayStatics.LoadGameFromSlot` "MainSlot"))
    (bind _asbp_save_data (cast `/Game/Blueprints/Save/BP_SaveData` _returnvalue_2))
    (set `self.SaveData` _asbp_save_data)
    (else
      (bind _returnvalue_3 (`GameplayStatics.CreateSaveGameObject` "/Game/Blueprints/Save/BP_SaveData.BP_SaveData_C"))
      (set `self.SaveData` _returnvalue_3))))

(event `SaveCheckpoint`
  (params (`New Checkpoint` :type Integer))
  (bind _savedata (`self.SaveData`))
  ;[1 1 1] Creating a SAVE GAME DATA in a Checkpoint
  (set `/Game/Blueprints/Save/BP_SaveData.checkpointNum` `New Checkpoint` _savedata)
  (`GameplayStatics.SaveGameToSlot` _savedata "MainSlot") ; Makes sure that the save game data is saved. \nIf the game is closed, there will be game data - a checkpoint
)

(event `Save Sensitivity`
  (params (`New Sensitivity` :type "Float (double-precision)"))
  (bind _savedata (`self.SaveData`))
  (set `/Game/Blueprints/Save/BP_SaveData.Sensitivity` `New Sensitivity` _savedata)
  (`GameplayStatics.SaveGameToSlot` _savedata "MainSlot"))

(event `SaveFinalGather`
  (params (`New Gather` :type "Float (double-precision)"))
  (bind _savedata (`self.SaveData`))
  (set `/Game/Blueprints/Save/BP_SaveData.FinalGather` `New Gather` _savedata)
  (`GameplayStatics.SaveGameToSlot` _savedata "MainSlot"))

(event `SaveSceneDetail`
  (params (`New Detail` :type "Float (double-precision)"))
  (bind _savedata (`self.SaveData`))
  (set `/Game/Blueprints/Save/BP_SaveData.SceneDetail` `New Detail` _savedata)
  (`GameplayStatics.SaveGameToSlot` _savedata "MainSlot"))