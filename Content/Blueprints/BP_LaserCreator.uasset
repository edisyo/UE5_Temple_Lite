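; Laser emitter that bounces off BPI_Reflective actors to activate a BP_LaserGoal, switchable through Activate/Deactivate events unless TurnLaserOn is set.
; Each tick it line-traces from its Arrow, continuing along the hit normal rather than a true reflection, up to BounceAmount bounces.
; BeginPlay pre-spawns a stretched mesh and Niagara spark per segment, shown or hidden as needed.
; Hitting a goal stops bouncing; losing it ends activation.
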(event `self.ReceiveBeginPlay`
  (bind _audio (`self.Audio`))
  ;[1 0.79 0.3571] To play or stop laser audio depending if laser is on/off (on start up)
  (if (`self.TurnLaserOn?`)
    (`AudioComponent.FadeIn` _audio 0.0 1.0 0.0 "Linear")
    (else
      (`AudioComponent.Stop` _audio)))
  (for _ (range (+ (`self.BounceAmount`) 1))
    ;[0.253 0.2303 0.3854] Create the Static Mesh & Particles used for LASERS
    ;;[1 0.763 0.5667] Create Mesh
    (bind _returnvalue (`|SpawnActorFromClass` "/Script/Engine.StaticMeshActor" (`SceneComponent.K2_GetComponentToWorld` (`self.DefaultSceneRoot`)) "Undefined" "MultiplyWithRoot" self null))
    (`StaticMeshActor.SetMobility` _returnvalue "Movable") ; Needs to set this first, otherwise statis mesh wont be movable
    (`StaticMeshComponent.SetStaticMesh` (`StaticMeshActor.StaticMeshComponent` _returnvalue) "/Game/Meshes/SM_LaserMesh.SM_LaserMesh")
    (`KismetArrayLibrary.Array_Add` (`self.LaserMeshes`) _returnvalue) ; Add each LaserMesh to an array
    ;;[1 0.5521 0.5521] Create Sparks
    (bind _returnvalue_2 (`NiagaraFunctionLibrary.SpawnSystemAttached` "/Game/Particles/NS_Spark.NS_Spark" (`self.DefaultSceneRoot`) "None" (0.0 0.0 0.0) (struct) "KeepRelativeOffset"))
    (`SceneComponent.SetHiddenInGame` _returnvalue_2 true false) ; Hide particle systems
    (`KismetArrayLibrary.Array_Add` (`self.LaserParticles`) _returnvalue_2)))

(event `/Game/Blueprints/BPI_Activatable.Activate`
  ;[0.4241 0.4844 0.2665] BPI functions
  (set `self.ActivateLaser?` true)
  ;;[0.609 0.6856 1] Sound on/off on activation/ deactivation
  (`AudioComponent.FadeIn` (`self.Audio`) 0.1 1.0 0.0 "Linear"))

(event `/Game/Blueprints/BPI_Activatable.Deactivate`
  ;[0.4241 0.4844 0.2665] BPI functions
  (set `self.ActivateLaser?` false)
  ;;[0.609 0.6856 1] Sound on/off on activation/ deactivation
  (`AudioComponent.FadeOut` (`self.Audio`) 0.1 0.0 "Linear"))

(event `self.ReceiveTick`
  (params (DeltaSeconds :type "Float (single-precision)"))
  (bind _arrow (`self.Arrow`))
  (bind _currentgoalsphere (`self.CurrentGoalSphere`))
  (bind _currentgoalsphere_2 (`self.CurrentGoalSphere`))
  (bind (_bblockinghit _binitialoverlap _time _distance _location _impactpoint _normal _impactnormal _physmat _hitactor) (`GameplayStatics.BreakHitResult` (`self.PreviousHit`)))
  ;[1 1 1] Raycast every tick - First Trace!!!
  (if (`self.TurnLaserOn?`)
    ;;[1 0.4122 0.3625] Reset these variable every frame
    (set `self.IsActivatingGoal?` false :!label _label)
    (set `self.PreviousHit` (struct))
    ;;[0.2543 0.6476 1] Index 0 becouse this is the FIRST trace !
    (`self.BounceLaser` (`SceneComponent.K2_GetComponentLocation` _arrow) (`SceneComponent.GetForwardVector` _arrow))
    (`self.Check if Hitting Goal`)
    (for _index (range 1 (+ (`self.BounceAmount`) 1))
      ;[1 1 1] How many bounces to calculate? - ALL THE OTHER TRACES
      ;;[1 1 1] Calculate bounces
      ;;;[0.3361 0.526 0.3799 1 12] IF the hit BP actor has a 'reflective' Blueprint Interface, then proceed
      (if (and (`self.PreviousReturn`) (`KismetSystemLibrary.DoesImplementInterface` _hitactor "/Game/Blueprints/BPI_Reflective.BPI_Reflective_C"))
        (`self.BounceLaser` _location _normal _index)
        (`self.Check if Hitting Goal`)
        (else
          ;;;[0.1927 0.0813 0.0813 1 14] Get the LaserMesh from the current LOOP and HIDE, if the trace is false!
          (`self.Hide Laser Mesh & Particle` _index))))
    ;;[1 1 1] END actiavtion if not hitting LaserGoal
    (if (not (`self.IsActivatingGoal?`))
      (`/Engine/EditorBlueprintResources/StandardMacros.IsValid` _currentgoalsphere
        (:`Is Valid`
          (`/Game/Blueprints/BP_LaserGoal.EndACtivation` _currentgoalsphere)
          (set `self.CurrentGoalSphere` null) ; set it back to null
        )))
    (elif (`self.ActivateLaser?`)
      (goto _label)
      (else
        ;;[1 0.3542 0.6649] Hide All Light Meshes
        (for _index_2 (range (+ (`self.BounceAmount`) 1))
          (`self.Hide Laser Mesh & Particle` _index_2))
        ;;[1 0.3594 0.3594] If not activated - stop lasers and goal actiavtion
        (`/Engine/EditorBlueprintResources/StandardMacros.IsValid` _currentgoalsphere_2
          (:`Is Valid`
            (`/Game/Blueprints/BP_LaserGoal.EndACtivation` _currentgoalsphere_2)
            (set `self.CurrentGoalSphere` null) ; set it back to null
          ))))))

(fn `Add Laser Mesh & Particle`
  (params (StartLocation :type "Vector Structure (by ref)") (EndLocation :type "Vector Structure (by ref)") (Normal :type "Vector Structure") (Index :type Integer))
  (bind _output (`|GetArrayItem` (`self.LaserMeshes`) Index))
  (bind _output_2 (`|GetArrayItem` (`self.LaserParticles`) Index))
  (bind _staticmeshcomponent (`StaticMeshActor.StaticMeshComponent` _output))
  ;[1 1 1] Draw the laser - FOR ALL OTHER TRACES
  (`self.SetActorHiddenInGame` _output false) ; UNHIDE  LaserMesh when it is put in the place correctly
  (`SceneComponent.K2_SetWorldLocationAndRotation` _staticmeshcomponent StartLocation (`KismetMathLibrary.FindLookAtRotation` StartLocation EndLocation) false false)
  (`SceneComponent.SetRelativeScale3D` _staticmeshcomponent (`KismetMathLibrary.MakeVector` (/ (`KismetMathLibrary.Vector_Distance` EndLocation StartLocation) 10.0) 1.0 1.0)) ; Set scale for laser mesh
  (`SceneComponent.K2_SetWorldLocationAndRotation` _output_2 (`local.EndLocation`) (`KismetMathLibrary.MakeRotFromX` (`local.Normal`)) false false)
  (`SceneComponent.SetHiddenInGame` _output_2 false false))

(fn `BounceLaser`
  (params (StartLocation :type "Vector Structure") (Direction :type "Vector Structure") (Index :type Integer))
  (bind (_bblockinghit _binitialoverlap _time _distance _location _impactpoint _normal _impactnormal _physmat _hitactor) (`GameplayStatics.BreakHitResult` (`self.PreviousHit`)))
  (bind (_bblockinghit_2 _binitialoverlap_2 _time_2 _distance_2 _location_2 _impactpoint_2 _normal_2 _impactnormal_2 _physmat_2 _hitactor_2 _hitcomponent _hitbonename _bonename _hititem _elementindex _faceindex _tracestart) (`GameplayStatics.BreakHitResult` (`self.PreviousHit`)))
  (bind (_bblockinghit_3 _binitialoverlap_3 _time_3 _distance_3 _location_3 _impactpoint_3 _normal_3 _impactnormal_3 _physmat_3 _hitactor_3 _hitcomponent_2 _hitbonename_2 _bonename_2 _hititem_2 _elementindex_2 _faceindex_2 _tracestart_2 _traceend) (`GameplayStatics.BreakHitResult` (`self.PreviousHit`)))
  ;[1 1 1] CALCULATE bounces
  (bind (_outhit _returnvalue) (`KismetSystemLibrary.LineTraceSingle` StartLocation (+ StartLocation (* Direction (`self.LaserLength`))) "TraceTypeQuery1" false (`|MakeArray` _hitactor) "None" true (struct :`R` 1.0 :`A` 1.0) (struct :`G` 1.0 :`A` 1.0) 0.0)) ; Trace inside the loop
  ;;[1 1 1] Assign Out/hit values for the First Trace
  (set `self.PreviousHit` _outhit) ; This now is the previous trace
  (set `self.PreviousReturn` _returnvalue)
  (`/Engine/EditorBlueprintResources/StandardMacros.IsValid` _hitactor
    (:`Is Valid`
      ;[0.5956 1 0.5852] if trace DOES HITS something - DRAW the laser
      (`self.Add Laser Mesh & Particle` _tracestart _location_2 _normal_2 (`local.Index`)))
    (:`Is Not Valid`
      ;[1 0.4372 0.3474] if trace DOES NOT HITS something - DRAW the laser
      (`self.Add Laser Mesh & Particle` _tracestart_2 _traceend _normal_3 (`local.Index`)))))

(fn `Check if Hitting Goal`
  (locals (LastHitLaserGoal :type "/Game/Blueprints/BP_LaserGoal Object Reference"))
  (bind _asbp_laser_goal (cast `/Game/Blueprints/BP_LaserGoal` (`.HitActor` (`GameplayStatics.BreakHitResult` (`self.PreviousHit`)))))
  ;[1 1 1] IF the LASER GOAL is hit, then stop bouncing lasers
  (`/Game/Blueprints/BP_LaserGoal.StartACtivation` _asbp_laser_goal)
  (set `self.PreviousReturn` false)
  (set `self.CurrentGoalSphere` _asbp_laser_goal)
  (set `self.IsActivatingGoal?` true))

(fn `Hide Laser Mesh & Particle`
  (params (Index :type Integer))
  (`self.SetActorHiddenInGame` (`|GetArrayItem` (`self.LaserMeshes`) Index) true)
  (`SceneComponent.SetHiddenInGame` (`|GetArrayItem` (`self.LaserParticles`) Index) true false))

(fn `UserConstructionScript`)