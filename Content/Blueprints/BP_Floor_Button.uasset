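; Floor pressure button that is pressed by the first-person character or physics-simulating objects overlapping its collision box.
; Overlap plays a timeline press animation with looping sound and sends BPI_Activatable messages to its target objects.
; On end overlap it releases and deactivates them only if no player or physics object remains.
; With UseMultipleButtons, ActivateMultiple checks linked buttons and activates UniqueObjects only when all are pressed, otherwise deactivating them.
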(event `self.Collision_box.OnComponentBeginOverlap`
  (params (OverlappedComponent :type "PrimitiveComponent Object Reference") (OtherActor :type "Actor Object Reference") (OtherComp :type "PrimitiveComponent Object Reference") (OtherBodyIndex :type Integer) (bFromSweep :type Boolean) (SweepResult :type "HitResult Structure (by ref)"))
  ;[0.401 0.401 0.401] Button ON / OFF
  ;;[0.5515 1 0.4912 1 16] Check if player or an object that simulates physics collides with this collider
  (if (or (== (`GameplayStatics.GetObjectClass` OtherActor) "/Game/Blueprints/BP_FirstPersonCharacter.BP_FirstPersonCharacter_C") (`SceneComponent.IsSimulatingPhysics` OtherComp "None"))
    (set `self.ButtonActivated` true)
    (`self.Button_down`)
    (`self.ActivateMultiple`)
    ;[1 1 1] Activating BPI functions
    (for _array_element (`self.ActivateObjects`)
      (if (`KismetSystemLibrary.DoesImplementInterface` _array_element "/Game/Blueprints/BPI_Activatable.BPI_Activatable_C")
        (message `/Game/Blueprints/BPI_Activatable.Activate` _array_element)))))

(event `Button_down`
  ;[1 0.6406 0.6406] Button Down Animation
  (`AudioComponent.FadeIn` (`self.PushRock_loop`) 0.05 0.2 0.0 "Linear")
  (bind (_direction _z_offset) (`Timeline|Button_Press_Animation` :!label _label)
    (:`Update`
      (`SceneComponent.K2_SetRelativeLocation` (`self.Button`) (`KismetMathLibrary.MakeVector` 0.0 0.0 _z_offset) false false))
    (:`Finished`
      (`AudioComponent.FadeOut` (`self.PushRock_loop`) 0.05 0.0 "Linear"))))

(event `Button_up`
  ;[1 0.6406 0.6406] Button Down Animation
  (`AudioComponent.FadeIn` (`self.PushRock_loop`) 0.05 0.2 0.0 "Linear")
  (goto _label :!via `Reverse`))

(event `self.Collision_box.OnComponentEndOverlap`
  (params (OverlappedComponent :type "PrimitiveComponent Object Reference") (OtherActor :type "Actor Object Reference") (OtherComp :type "PrimitiveComponent Object Reference") (OtherBodyIndex :type Integer))
  ;[0.401 0.401 0.401] Button ON / OFF
  ;;[0.5515 1 0.4912 1 16] Check if player or an object that simulates physics collides with this collider
  (if (and (or (== (`GameplayStatics.GetObjectClass` OtherActor) "/Game/Blueprints/BP_FirstPersonCharacter.BP_FirstPersonCharacter_C") (`SceneComponent.IsSimulatingPhysics` OtherComp "None")) (`self.NothingOnButton`))
    (set `self.ButtonActivated` false)
    (`self.Button_up`)
    (`self.ActivateMultiple`)
    ;[1 1 1] Activating BPI functions
    (for _array_element (`self.ActivateObjects`)
      (if (`KismetSystemLibrary.DoesImplementInterface` _array_element "/Game/Blueprints/BPI_Activatable.BPI_Activatable_C")
        (message `/Game/Blueprints/BPI_Activatable.Deactivate` _array_element)))))

(fn `ActivateMultiple`
  (bind _objectstoactivateunique (`self.ObjectsToActivateUnique`))
  ;[1 1 1] OLD BP, after splitting level into multiple - suddenly dont work...
  (if (`self.UseMultipleButtons`)
    (for _index (range (+ (`KismetArrayLibrary.Array_Length` _objectstoactivateunique) 1))
      ;;[1 0.8399 0.1063] if even one button in loop isnt activated, break the loop and start again - if all are activated, the loop wont break and will set AllActorsActivated true and will move on with Loops Completed node
      (bind _asbp_floor_button (cast `/Game/Blueprints/BP_Floor_Button` (`|GetArrayItem` _objectstoactivateunique _index)))
      (if (`/Game/Blueprints/BP_Floor_Button.ButtonActivated` _asbp_floor_button)
        (set `self.AllActorsActivated` true)
        (else
          (set `self.AllActorsActivated` false)
          (break))))
    (if (`self.AllActorsActivated`)
      (for _array_element (`self.UniqueObjects`)
        (message `/Game/Blueprints/BPI_Activatable.Activate` _array_element))
      (else
        (for _array_element_2 (`self.UniqueObjects`)
          (message `/Game/Blueprints/BPI_Activatable.Deactivate` _array_element_2))))))

(fn `NothingOnButton`
  (returns (Return :type Boolean))
  (locals (`IsPhysicsObjectsOnButton?` :type Boolean))
  (bind _collision_box (`self.Collision_box`))
  ;[1 1 1] Check for physics objects on top of button
  (for _array_element (`PrimitiveComponent.GetOverlappingComponents` _collision_box)
    (if (`SceneComponent.IsSimulatingPhysics` _array_element "None")
      (set `local.IsPhysicsObjectsOnButton?` true)))
  (return (and (== (`KismetArrayLibrary.Array_Length` (`PrimitiveComponent.GetOverlappingActors` _collision_box "/Game/Blueprints/BP_FirstPersonCharacter.BP_FirstPersonCharacter_C")) 0) (not (`local.IsPhysicsObjectsOnButton?`)))))

(fn `UserConstructionScript`)